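; BP_MapEditorController tracks which input tool is active in the map editor, driven by held keys.
; On BeginPlay it enables input from player controller 0, then holding Z, X or C sets InputToolType to one of three enum values.
; Releasing any of these keys resets it to a shared fourth value, even if another is still held.
; GetToolType exposes the current tool to other Blueprints.
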(event `self.ReceiveBeginPlay`
  (`self.EnableInput` (`GameplayStatics.GetPlayerController` 0)))

(event `Key|Z`
  (params (Key :type "Key Structure"))
  (:`Pressed`
    (set `self.InputToolType` "NewEnumerator0"))
  (:`Released`
    (set `self.InputToolType` "NewEnumerator3" :!label _label)))

(event `Key|X`
  (params (Key :type "Key Structure"))
  (:`Pressed`
    (set `self.InputToolType` "NewEnumerator1"))
  (:`Released`
    (goto _label)))

(event `Key|C`
  (params (Key :type "Key Structure"))
  (:`Pressed`
    (set `self.InputToolType` "NewEnumerator2"))
  (:`Released`
    (goto _label)))

(fn `GetToolType`
  (returns (InputToolType :type "/Game/Project000/E_MapEditorFillToolType Enum"))
  (return (`self.InputToolType`)))

(fn `UserConstructionScript`)