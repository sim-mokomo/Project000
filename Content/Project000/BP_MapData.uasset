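; BP_MapData holds one stage map as a flat array of map-editor fill-tool enum values.
; Initialize loads the file at the given path and parses its comma-separated numeric tokens into that array.
; GetData and SetData address cells by X/Y using row-major indexing on MaxMapWidth, with SetData also printing the index.
; OutputRawMapData converts the array back into a comma-joined string, inserting an extra entry after each row.
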(event `Initialize`
  (params (FileFullPath :type String))
  (bind (_stagedata _exist) (`self.GetRawMapData`))
  (set `self.FileFullPath` FileFullPath)
  (if _exist
    (for _array_element (`KismetStringLibrary.ParseIntoArray` _stagedata ",")
      (if (`KismetStringLibrary.IsNumeric` _array_element)
        (`KismetArrayLibrary.Array_Add` (`self.EnumMapData`) (cast `/Game/Project000/E_MapEditorFillToolType` (`KismetMathLibrary.Conv_IntToByte` (`KismetStringLibrary.Conv_StringToInt` (`KismetStringLibrary.Trim` _array_element)))))))))

(fn `GetData`
  (params (IndexX :type Integer) (IndexY :type Integer))
  (returns (Data :type "/Game/Project000/E_MapEditorFillToolType Enum"))
  (return (`|GetArrayItem` (`self.EnumMapData`) (`self.GetIndex` IndexX IndexY))))

(fn `GetFileName`
  (returns (FileName :type String))
  (return (`BlueprintPathsLibrary.GetBaseFilename` (`self.FileFullPath`))))

(fn `GetIndex`
  (params (X :type Integer) (Y :type Integer))
  (returns (Index :type Integer))
  (return (+ X (* Y (`/Game/Project000/BP_MapEditorMacro.MaxMapWidth`)))))

(fn `GetMapData`
  (returns (EnumMapData :type "Array of /Game/Project000/E_MapEditorFillToolType Enum"))
  (return (`self.EnumMapData`)))

(fn `GetRawMapData`
  (returns (StageData :type String) (Exist :type Boolean))
  (bind (_result _returnvalue) (`FileFunctionLibrary.LoadFileToString` (`self.FileFullPath`)))
  (return _result _returnvalue))

(fn `OutputRawMapData`
  (returns (Output :type String))
  (locals (RawMapData :type "Array of String"))
  (for (_array_element _array_index) (`self.EnumMapData`)
    (`KismetArrayLibrary.Array_Add` (`local.RawMapData`) (`KismetStringLibrary.Conv_IntToString` (`KismetMathLibrary.Conv_ByteToInt` _array_element)))
    (if (and (== (mod (+ _array_index 1) (`/Game/Project000/BP_MapEditorMacro.MaxMapWidth`)) 0) true)
      (`KismetArrayLibrary.Array_Add` (`local.RawMapData`) " \n")))
  (return (`KismetStringLibrary.Concat_StrStr` "," (`KismetStringLibrary.JoinStringArray` (`local.RawMapData`) ","))))

(fn `SetData`
  (params (X :type Integer) (Y :type Integer) (Item :type "/Game/Project000/E_MapEditorFillToolType Enum (by ref)" :default "NewEnumerator3"))
  (bind _index (`self.GetIndex` X Y))
  (`KismetSystemLibrary.PrintString` null (`KismetStringLibrary.Conv_IntToString` _index))
  (`KismetArrayLibrary.Array_Set` (`self.EnumMapData`) _index Item))