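; BP_Stage is a grid stage that builds a cube-based level from map data, loading map "000" in its construction script.
; Load adds a static mesh component per cell, spaced by the cube's bounds, and records components and cell types in flat row-major arrays.
; SetVisibility shows only Wall cells, while getters expose block type by X/Y and world position by index.
; GetMapBlockCenterPosition is an empty stub.
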(event `Clear`
  (`KismetArrayLibrary.Array_Clear` (`self.StageBlocks`))
  (`KismetArrayLibrary.Array_Clear` (`self.StageTypes`)))

(event `Load`
  (params (MapData :type "/Game/Project000/BP_MapData Object Reference"))
  (set `self.CurrentReadingMapData` MapData)
  (`self.Clear`)
  (for _index (range (`self.Height`))
    (for _index_2 (range (`/Game/Project000/BP_MapEditorMacro.MaxMapWidth`))
      (bind _returnvalue (`AddComponent|NODE_AddStaticMeshComponent-3` :`RelativeTransform` (`KismetMathLibrary.MakeTransform` (`KismetMathLibrary.MakeVector` (* _index_2 (* 2 (.x (`.Max` (break `Box` (`StaticMesh.GetBoundingBox` (`self.MapCubeMesh`))))))) (* _index (* 2 (.y (`.Max` (break `Box` (`StaticMesh.GetBoundingBox` (`self.MapCubeMesh`)))))))))))
      (`StaticMeshComponent.SetStaticMesh` _returnvalue (`self.MapCubeMesh`))
      (`KismetArrayLibrary.Array_Add` (`self.StageBlocks`) _returnvalue)
      (bind _data (`/Game/Project000/BP_MapData.GetData` MapData _index_2 _index))
      (`KismetArrayLibrary.Array_Add` (`self.StageTypes`) _data)
      (`self.SetVisibility` _index_2 _index _data))))

(event `SetVisibility`
  (params (X :type Integer) (Y :type Integer) (Type :type "/Game/Project000/E_MapEditorFillToolType Enum" :default "NewEnumerator3"))
  (bind _output (`|GetArrayItem` (`self.StageBlocks`) (`self.ConvertToIndex` X Y)))
  (switch `/Game/Project000/E_MapEditorFillToolType` Type
    (:`NewEnumerator3`
      (`SceneComponent.SetVisibility` _output false false :!label _label))
    (:`NewEnumerator0`
      (goto _label))
    (:`NewEnumerator1`
      (`SceneComponent.SetVisibility` _output true false))
    (:`NewEnumerator2`
      (goto _label))))

(fn `ConvertToIndex`
  (params (X :type Integer) (Y :type Integer))
  (returns (Index :type Integer))
  (return (+ X (* Y (`/Game/Project000/BP_MapEditorMacro.MaxMapWidth`)))))

(fn `GetBlockPosition`
  (params (Index :type Integer))
  (returns (Position :type "Vector Structure"))
  (return (`SceneComponent.K2_GetComponentLocation` (`|GetArrayItem` (`self.StageBlocks`) Index))))

(fn `GetBlockType`
  (params (X :type Integer) (Y :type Integer))
  (returns (BlockType :type "/Game/Project000/E_MapEditorFillToolType Enum"))
  (return (`|GetArrayItem` (`self.StageTypes`) (`self.ConvertToIndex` X Y))))

(fn `GetMapBlockCenterPosition`
  (params (NewParam :type Integer) (NewParam1 :type Integer)))

(fn `UserConstructionScript`
  (bind _returnvalue (`|GenericCreateObject` "/Game/Project000/BP_MapData.BP_MapData_C" self))
  (`/Game/Project000/BP_MapData.Initialize` _returnvalue (`/Game/Project000/BP_MapEditorMacro.CreatePathToMapData` "000"))
  (`self.Load` _returnvalue))