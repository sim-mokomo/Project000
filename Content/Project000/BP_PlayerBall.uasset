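; BP_PlayerBall is a player-controlled ball that glides toward a target location and tracks clamped X/Y map indices.
; Tick lerps the actor toward DistMoveLocation with sweep, and IsMoving compares the remaining distance to a threshold.
; Four directional inputs call CheckMovable to choose a new target.
; CheckMovable is unfinished: it runs a debug-drawn line trace but ignores the hits and never sets a result, so input moves nothing.
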(event `UpdateLocation`
  (`self.K2_SetActorLocation` (`KismetMathLibrary.VLerp` (`self.K2_GetActorLocation`) (`self.DistMoveLocation`) (`self.DistMoveLerpSpeed`)) true))

(event `self.ReceiveTick`
  (params (DeltaSeconds :type "Float (single-precision)"))
  (`self.UpdateLocation`))

(event `Initialize`
  (params (X :type Integer) (Y :type Integer) (StartPos :type "Vector Structure"))
  (`self.K2_SetActorLocation` StartPos)
  (set `self.X` X)
  (set `self.Y` Y))

(event `self.ReceiveBeginPlay`
  (set `self.DistMoveLocation` (`self.K2_GetActorLocation`))
  (`self.EnableInput` (`GameplayStatics.GetPlayerController` 0)))

(event `InputAction|MoveDown`
  (params (Key :type "Key Structure"))
  (:`Pressed`
    (`self.CheckAndMove` (-1.0 0.0 0.0))))

(event `InputAction|MoveUp`
  (params (Key :type "Key Structure"))
  (:`Pressed`
    (`self.CheckAndMove` (1.0 0.0 0.0))))

(event `CheckAndMove`
  (params (CheckDirection :type "Vector Structure"))
  (bind (_movable _distmovelocation) (`self.CheckMovable` CheckDirection))
  (if _movable
    (set `self.DistMoveLocation` _distmovelocation)))

(event `InputAction|MoveLeft`
  (params (Key :type "Key Structure"))
  (:`Pressed`
    (`self.CheckAndMove` (0.0 -1.0 0.0))))

(event `MovementPerBlock`
  (params (diffX :type Integer) (diffY :type Integer))
  (set `self.X` (`KismetMathLibrary.Clamp` (+ (`self.X`) diffX) 0 (- (`/Game/Project000/BP_MapEditorMacro.MaxMapWidth`) 1)))
  (set `self.Y` (`KismetMathLibrary.Max` (+ (`self.Y`) diffY))))

(event `InputAction|MoveRight`
  (params (Key :type "Key Structure"))
  (:`Pressed`
    (`self.CheckAndMove` (0.0 1.0 0.0))))

(event `SetDistMoveLocation`
  (params (Dist :type "Vector Structure"))
  (set `self.DistMoveLocation` Dist))

(fn `CheckMovable`
  (params (CheckDirection :type "Vector Structure"))
  (returns (Movable :type Boolean) (DistMoveLocation :type "Vector Structure"))
  (bind _returnvalue (`self.K2_GetActorLocation`))
  (bind _outhits (`KismetSystemLibrary.LineTraceMultiForObjects` :`Start` _returnvalue :`End` (+ _returnvalue (* CheckDirection 9999.0)) :`ObjectTypes` (`|MakeArray` "ObjectTypeQuery1" "ObjectTypeQuery2" :!type "EObjectTypeQuery Enum") :`DrawDebugType` "ForDuration" :`DrawTime` 1.0))
  (for _array_element _outhits
    _))

(fn `GetIndexes`
  (returns (X :type Integer) (Y :type Integer))
  (return (`self.X`) (`self.Y`)))

(fn `IsMoving`
  (returns (IsMoving :type Boolean))
  (return (> (`KismetMathLibrary.VSize` (- (`self.DistMoveLocation`) (`self.K2_GetActorLocation`))) (`self.AsMovingThrethhold`))))

(fn `UserConstructionScript`)